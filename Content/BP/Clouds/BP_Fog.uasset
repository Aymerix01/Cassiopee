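; BP_Fog fills a rectangular area around itself with a grid of Cloud actors when play begins.
; BeginPlay first destroys one existing Cloud if found, then loops over GridSize at Gap spacing, centred on the actor.
; Each Cloud spawns with a random quarter-turn yaw and a random uniform scale between MinScale and MaxScale.
; Every spawn calls AddPollutionFog on the PollutionManager.
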(event EventBeginPlay
  (bind _gridsize (Variables|Default|GetGridSize))
  (bind _gap (Variables|Default|GetGap))
  (bind _returnvalue (Utilities|Operators|Divide (.y _gridsize) 2.0 _gap))
  (bind _returnvalue_2 (Utilities|Operators|Divide (.x _gridsize) 2.0 _gap))
  (bind _returnvalue_3 (Actor|GetActorOfClass "/Game/BP/Clouds/Cloud.Cloud_C"))
  (Utilities|IsValid _returnvalue_3
    (:Is%20Valid
      (Actor|DestroyActor _returnvalue_3))
    (:Is%20Not%20Valid
      _))
  (for _index (range (Math|Float|Truncate (* _returnvalue_2 -1.0)) (Math|Float|Truncate _returnvalue_2))
    (for _index_2 (range (Math|Float|Truncate (* _returnvalue -1.0)) (Math|Float|Truncate _returnvalue))
      (Game|SpawnActorfromClass "/Game/BP/Clouds/Cloud.Cloud_C" (Math|Transform|MakeTransform (+ (Transformation|GetActorLocation) (Math|Vector|MakeVector (* _index (Variables|Default|GetGap)) (* _index_2 (Variables|Default|GetGap)) 0.0)) (Math|Rotator|MakeRotator 0.0 0.0 (* (Math|Random|RandomIntegerinRange 0 4) 9e+01)) (Math|Conversions|ToVector(Float) (Math|Random|RandomFloatinRange (Variables|Default|GetMinScale) (Variables|Default|GetMaxScale)))) "Undefined" "MultiplyWithRoot" 0 0)
      (Default|AddPollutionFog (Variables|Default|GetPollutionManager)))))

(fn ConstructionScript)