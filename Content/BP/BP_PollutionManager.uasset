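; BP_PollutionManager tracks fog, waste and water pollution counts and reports them to the pollution widget in the top HUD.
; Fog and water counts move through add/remove events, while AddPollutionWaste recounts waste from a large box multi-trace and RemovePollutionWaste decrements it.
; BeginPlay runs that recount, then retries until the HUD widget is valid to initialise it.
; A delay-throttled Tick prints the counts and refreshes the widget.
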(event Custom|AddPollutionFog
  (Variables|Default|SetNumberPollutionFog (+ (Variables|Default|GetNumberPollutionFog) 1)))

(event Custom|AddPollutionWater
  (Variables|Default|SetNumberPollutionWater (+ (Variables|Default|GetNumberPollutionWater) 1)))

(event Custom|AddPollutionWaste
  (Variables|Default|SetNumberPollutionWaste 0)
  (bind _outhits (Class|KismetSystemLibrary|BoxTraceMulti "0, 0, 0" "0, 0, 0" "10000.000000,10000.000000,10000.000000" "0, 0, 0" "TraceTypeQuery5" false 0 "None" true))
  (Variables|Default|SetNumberPollutionWaste (+ (Variables|Default|GetNumberPollutionWaste) (Utilities|Array|Length _outhits))))

(event Custom|RemovePollutionWaste
  (Variables|Default|SetNumberPollutionWaste (- (Variables|Default|GetNumberPollutionWaste) 1)))

(event Custom|RemovePollutionFog
  (Variables|Default|SetNumberPollutionFog (- (Variables|Default|GetNumberPollutionFog) 1)))

(event Custom|RemovePollutionWater
  (Variables|Default|SetNumberPollutionWater (- (Variables|Default|GetNumberPollutionWater) 1)))

(event EventBeginPlay
  (Utilities|FlowControl|Delay 1.0)
  (CallFunction|AddPollutionWaste)
  (bind _asmain_hud (Utilities|Casting|CastToMainHud (HUD|GetHUD (Game|GetPlayerController 0))))
  (Utilities|IsValid (Variables|/Game/UI/MainHud.MainHud_C|GetTopHudWidget _asmain_hud) :!label _label
    (:Is%20Valid
      (Variables|Default|SetWBP%20Pollution%20Manager (Variables|/Game/UI/WBP_Main.WBP_Main_C|GetWBP_PollutionManager (Variables|/Game/UI/MainHud.MainHud_C|GetTopHudWidget _asmain_hud)))
      (Default|InitStartValues (Variables|Default|GetWBP%20Pollution%20Manager) (Math|Conversions|ToFloat(Integer) (Variables|Default|GetNumberPollutionFog)) (Math|Conversions|ToFloat(Integer) (Variables|Default|GetNumberPollutionWaste)) (Math|Conversions|ToFloat(Integer) (Variables|Default|GetNumberPollutionWater))))
    (:Is%20Not%20Valid
      (Utilities|FlowControl|Delay 1.0)
      (goto _label))))

(event EventTick
  (params (DeltaSeconds :type Float%20%28single-precision%29))
  (bind _wbp_pollution_manager (Variables|Default|GetWBP%20Pollution%20Manager))
  (Utilities|FlowControl|Delay 5.0)
  (Development|PrintText (Utilities|Text|FormatText "Fog : {fog}" (Utilities|String|ToString(Integer) (Variables|Default|GetNumberPollutionFog))) false)
  (Development|PrintText (Utilities|Text|FormatText "Waste : {waste}" (Utilities|String|ToString(Integer) (Variables|Default|GetNumberPollutionWaste))) false)
  (Development|PrintText (Utilities|Text|FormatText "Water : {water}" (Utilities|String|ToString(Integer) (Variables|Default|GetNumberPollutionWater))) false)
  (Development|PrintText "Pollution Manager : " false)
  (Utilities|IsValid _wbp_pollution_manager
    (:Is%20Valid
      (Default|UpdatePollutionUI _wbp_pollution_manager (Math|Conversions|ToFloat(Integer) (Variables|Default|GetNumberPollutionFog)) (Math|Conversions|ToFloat(Integer) (Variables|Default|GetNumberPollutionWaste)) (Math|Conversions|ToFloat(Integer) (Variables|Default|GetNumberPollutionWater))))))

(fn ConstructionScript)