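; BP_TerrainLimite is a terrain boundary actor that clears objects reaching its five box volumes.
; A Delay on Tick runs HitByChannel for each box roughly every five seconds, multi-box tracing from its location to that location with Z multiplied by 32.
; Every hit actor receives DestroyMessage with the PollutionManager, and those still valid and tagged Spawnable also trigger RemovePollutionWaste on the manager.
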(event EventTick
  (params (DeltaSeconds :type Float%20%28single-precision%29))
  (Utilities|FlowControl|Delay 5.0)
  (Utilities|FlowControl|Sequence
    (:then_0
      (CallFunction|HitbyChannel (Variables|Default|GetBox)))
    (:then_1
      (CallFunction|HitbyChannel (Variables|Default|GetBox1)))
    (:then_2
      (CallFunction|HitbyChannel (Variables|Default|GetBox2)))
    (:then_3
      (CallFunction|HitbyChannel (Variables|Default|GetBox3)))
    (:then_4
      (CallFunction|HitbyChannel (Variables|Default|GetBox4)))))

(fn ConstructionScript)

(fn HitbyChannel
  (params (BoxCollision :type Box%20Component%20Object%20Reference))
  (bind _returnvalue (Transformation|GetWorldLocation BoxCollision))
  (bind _pollutionmanager (Variables|Default|GetPollutionManager))
  (bind _outhits (Class|KismetSystemLibrary|BoxTraceMulti _returnvalue (* _returnvalue "1.000000,1.000000,32.000000") (* (Transformation|GetWorldScale BoxCollision) 32.0) (Transformation|GetWorldRotation BoxCollision) "TraceTypeQuery7" false 0 "None" true))
  (for _array_element _outhits
    (Class|BPITrash|Destroy(Message) (.HitActor (Collision|BreakHitResult _array_element)) _pollutionmanager)
    (Utilities|IsValid (.HitActor (Collision|BreakHitResult _array_element))
      (:Is%20Valid
        (if (Actor|ActorHasTag (.HitActor (Collision|BreakHitResult _array_element)) "Spawnable")
          (if true
            (Default|RemovePollutionWaste _pollutionmanager)))))))