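; Spawner actor that scatters water pollution actors over a rectangular area and counts them in the pollution manager.
; On BeginPlay it destroys the first existing WaterPollution actor it finds, then loops over a grid centered on itself, sized by GridSize and spaced by Gap.
; Each cell spawns a WaterPollution with random quarter-turn yaw and random horizontal scale, then calls AddPollutionWater on PollutionManager.
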(event EventBeginPlay
  (bind _gridsize (Variables|Default|GetGridSize))
  (bind _gap (Variables|Default|GetGap))
  (bind _minscale (Variables|Default|GetMinScale))
  (bind _maxscale (Variables|Default|GetMaxScale))
  (bind _returnvalue (Math|Random|RandomFloatinRange _minscale _maxscale))
  (bind _returnvalue_2 (Utilities|Operators|Divide (.y _gridsize) 2.0 _gap))
  (bind _returnvalue_3 (Utilities|Operators|Divide (.x _gridsize) 2.0 _gap))
  (bind _returnvalue_4 (Math|Conversions|ToVector(Float) _returnvalue))
  (bind _returnvalue_5 (Actor|GetActorOfClass "/Game/BP/Water/WaterPollution.WaterPollution_C"))
  (Utilities|IsValid _returnvalue_5
    (:Is%20Valid
      (Actor|DestroyActor _returnvalue_5))
    (:Is%20Not%20Valid
      _))
  (for _index (range (Math|Float|Truncate (* _returnvalue_3 -1.0)) (Math|Float|Truncate _returnvalue_3))
    (for _index_2 (range (Math|Float|Truncate (* _returnvalue_2 -1.0)) (Math|Float|Truncate _returnvalue_2))
      (Game|SpawnActorfromClass "/Game/BP/Water/WaterPollution.WaterPollution_C" (Math|Transform|MakeTransform (+ (Transformation|GetActorLocation) (Math|Vector|MakeVector (* _index (Variables|Default|GetGap)) (* _index_2 (Variables|Default|GetGap)) 0.0)) (Math|Rotator|MakeRotator 0.0 0.0 (* (Math|Random|RandomIntegerinRange 0 4) 9e+01)) (Math|Vector|MakeVector (.x _returnvalue_4) (.y _returnvalue_4) 1.0)) "Undefined" "MultiplyWithRoot" 0 0)
      (Default|AddPollutionWater (Variables|Default|GetPollutionManager)))))

(fn ConstructionScript)