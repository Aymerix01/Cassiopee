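; AC_PollutionWatcher is a building component that switches on the pollution HUD display and the effects of a pollution watcher building.
; On BeginPlay it caches the pollution manager widget from the top HUD widget of the player's MainHud.
; InitPollutionWatcher initializes that widget's visibility, then activates the Niagara effect on its CB_BuildingPW owner without resetting it.
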(event Custom|InitPollutionWatcher
  (Default|InitVisibility (Variables|Default|GetWBP%20Pollution%20Manager))
  (bind _ascb_building_pw (Utilities|Casting|CastToCB_BuildingPW (Components|GetOwner)))
  (Components|Activation|Activate (Variables|/Game/BP/Building/CB_BuildingPW.CB_BuildingPW_C|GetNiagara _ascb_building_pw) false))

(event EventBeginPlay
  (bind _asmain_hud (Utilities|Casting|CastToMainHud (HUD|GetHUD (Game|GetPlayerController 0))))
  (Variables|Default|SetWBP%20Pollution%20Manager (Variables|/Game/UI/WBP_Main.WBP_Main_C|GetWBP_PollutionManager (Variables|/Game/UI/MainHud.MainHud_C|GetTopHudWidget _asmain_hud))))