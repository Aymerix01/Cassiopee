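; Actor component for buildings that spawns Korogu entities around its owner.
; On begin play it caches the level's entities controller, printing an error if none exists.
; SpawnKorogu spawns a configured number of BP_Entity pawns at random offsets within range at fixed height.
; Each spawn registers its AI controller with the entities controller, refreshes the HUD entity counter and activates the building's Niagara effect.
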(event Custom|SpawnKorogu
  (bind _returnvalue (Math|Random|RandomUnitVector))
  (bind _returnvalue_2 (Components|GetOwner))
  (bind _range (Variables|Default|GetRange))
  (bind _returnvalue_3 (Math|Random|RandomFloatinRange 1e+02 _range))
  (bind _returnvalue_4 (Transformation|GetActorLocation _returnvalue_2))
  (bind _returnvalue_5 (* _returnvalue _returnvalue_3))
  (bind _returnvalue_6 (+ _returnvalue_5 _returnvalue_4))
  (bind (_x _y) (Math|Vector|BreakVector _returnvalue_6))
  (for _index (range 1 (Variables|Default|GetKoroguToSpawn))
    (bind _returnvalue_7 (AI|SpawnAIFromClass "/Game/BP/Entity/BP_Entity.BP_Entity_C" 0 (Math|Vector|MakeVector _x _y 1.5e+02) "0, 0, 0" true 0))
    (Utilities|IsValid _returnvalue_7
      (:Is%20Valid
        (bind _asbp_entity_controller (Utilities|Casting|CastToBP_EntityController (Pawn|GetController _returnvalue_7)))
        (Utilities|Array|Add (Variables|/Game/BP/Entity/BP_EntitiesController.BP_EntitiesController_C|GetEntitiesControllerSpawned (Variables|Default|GetEntities%20controller)) _asbp_entity_controller)
        (bind _asmain_hud (Utilities|Casting|CastToMainHud (HUD|GetHUD (Game|GetPlayerController 0))))
        (Default|UpdateNbrEntities (Variables|/Game/UI/WBP_Main.WBP_Main_C|GetWBP_NbrEntities (Variables|/Game/UI/MainHud.MainHud_C|GetTopHudWidget _asmain_hud)))
        (bind _ascb_building_ph (Utilities|Casting|CastToCB_BuildingPH (Components|GetOwner)))
        (Components|Activation|Activate (Variables|/Game/BP/Building/CB_BuildingPH.CB_BuildingPH_C|GetNiagara _ascb_building_ph) false)))))

(event EventBeginPlay
  (bind _returnvalue (Actor|GetActorOfClass "/Game/BP/Entity/BP_EntitiesController.BP_EntitiesController_C"))
  (bind _output_get (Variables|Default|SetEntities%20controller _returnvalue))
  (Utilities|IsValid _output_get
    (:Is%20Not%20Valid
      (Development|PrintString "error"))))