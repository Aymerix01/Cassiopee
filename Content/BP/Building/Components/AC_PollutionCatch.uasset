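; Actor component in the building system that moves its owning actor toward a given position, then destroys it.
; MovementBeforeDestruction stores the target, enables movement and destroys the owner after a fixed delay, whether or not it has arrived.
; While movement is enabled, Tick eases the owner toward the target with VInterpTo and no sweep.
; BeginPlay records the start location, which the graph never reads.
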(event Custom|MovementBeforeDestruction
  (params (Position :type Vector))
  (Variables|Default|SetEndPos Position)
  (Variables|Default|SetStartMvmt true)
  (Utilities|FlowControl|Delay 4.0)
  (Actor|DestroyActor (Components|GetOwner)))

(event EventTick
  (params (DeltaSeconds :type Float%20%28single-precision%29))
  (if (Variables|Default|GetStartMvmt)
    (Transformation|SetActorLocation (Components|GetOwner) (Math|Interpolation|VInterpTo (Transformation|GetActorLocation (Components|GetOwner)) (Variables|Default|GetEndPos) DeltaSeconds 1.0) false false)))

(event EventBeginPlay
  (Variables|Default|SetStartPos (Transformation|GetActorLocation (Components|GetOwner))))