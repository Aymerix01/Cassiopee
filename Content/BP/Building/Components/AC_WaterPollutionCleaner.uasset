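; Building component that clears water pollution around its owner, firing the Niagara effect on CB_BuildingWFP owners.
; BeginPlay caches the owning building and all Chunk actors as the trace ignore list.
; CheckWaterPollution, once the building is placed and constructed, repeats a large upward sphere trace while it finds hits.
; Each pass messages the hit actor to clear its pollution and has the passed-in PollutionManager remove water pollution.
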(event Custom|CheckWaterPollution
  (params (PollutionManager :type BP%20Pollution%20Manager%20Object%20Reference))
  (bind _returnvalue (Components|GetOwner))
  (bind _returnvalue_2 (Components|GetOwner))
  (bind _building (Variables|Default|GetBuilding))
  (bind _returnvalue_3 (Transformation|GetActorLocation _returnvalue_2))
  (bind _returnvalue_4 (Transformation|GetActorLocation _returnvalue))
  (if (and (Variables|/Game/BP/Building/CB_BuildingAsset.CB_BuildingAsset_C|GetIsPlaced _building) (Variables|/Game/BP/Building/CB_BuildingAsset.CB_BuildingAsset_C|GetIsConstructed _building))
    (bind _returnvalue_5 (Collision|SphereTraceByChannel (+ _returnvalue_3 "") (+ _returnvalue_3 "0.000000,0.000000,500.000000") 9e+02 "TraceTypeQuery6" false (Variables|Default|GetChunkActors) "None"))
    (Variables|Default|SetTraceFindsCloud _returnvalue_5)
    (while (Variables|Default|GetTraceFindsCloud)
      (bind (_outhit _returnvalue_6) (Collision|SphereTraceByChannel (+ _returnvalue_4 "") (+ _returnvalue_4 "0.000000,0.000000,500.000000") 9e+02 "TraceTypeQuery6" false (Variables|Default|GetChunkActors) "None"))
      (Variables|Default|SetTraceFindsCloud _returnvalue_6)
      (Class|BPIWaterPollution|ClearWaterPollution(Message) (.HitActor (Collision|BreakHitResult _outhit)))
      (Default|RemovePollutionWater PollutionManager)
      (bind _ascb_building_wfp (Utilities|Casting|CastToCB_BuildingWFP (Components|GetOwner)))
      (Components|Activation|Activate (Variables|/Game/BP/Building/CB_BuildingWFP.CB_BuildingWFP_C|GetNiagara _ascb_building_wfp) false))))

(event EventBeginPlay
  (bind _ascb_building_asset (Utilities|Casting|CastToCB_BuildingAsset (Components|GetOwner)))
  (Variables|Default|SetBuilding _ascb_building_asset)
  (bind _outactors (Actor|GetAllActorsOfClass "/Game/BP/Landscape/Chunk.Chunk_C"))
  (Variables|Default|SetChunkActors _outactors))