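; Building component that makes a placed, constructed building periodically catch nearby pollution.
; A one-time multi-sphere trace, ignoring Chunk actors, fills the list of targets.
; After each delay, the last entry gets an AC_PollutionCatch component that moves it above the building, and PollutionManager's waste is decremented.
; The owner's yaw eases along the pollution-to-building direction; only CB_BuildingPP owners activate Niagara, as the CB_BuildingNet activation is unwired.
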(event EventBeginPlay
  (bind _ascb_building_asset (Utilities|Casting|CastToCB_BuildingAsset (Components|GetOwner)))
  (Variables|Default|SetBuilding _ascb_building_asset)
  (bind _asbp_player_controller_new (Utilities|Casting|CastToBP_PlayerControllerNew (Game|GetPlayerController 0)))
  (Variables|Default|SetPollution%20Manager (Variables|/Game/BP/Core/BP_PlayerControllerNew.BP_PlayerControllerNew_C|GetPollutionManager _asbp_player_controller_new)))

(event EventTick
  (params (DeltaSeconds :type Float%20%28single-precision%29))
  (bind _returnvalue (Components|GetOwner))
  (bind _returnvalue_2 (Components|GetOwner))
  (bind _building (Variables|Default|GetBuilding))
  (bind _pollutioninrange (Variables|Default|GetPollutionInRange))
  (bind _pollutioninrange_2 (Variables|Default|GetPollutionInRange))
  (bind _returnvalue_3 (Utilities|Array|Length _pollutioninrange_2))
  (bind _returnvalue_4 (Transformation|GetActorLocation _returnvalue))
  (bind _returnvalue_5 (- _returnvalue_3 1))
  (bind _output (Utilities|Array|Get(acopy) _pollutioninrange _returnvalue_5))
  (if (and (Variables|/Game/BP/Building/CB_BuildingAsset.CB_BuildingAsset_C|GetIsPlaced _building) (Variables|/Game/BP/Building/CB_BuildingAsset.CB_BuildingAsset_C|GetIsConstructed _building))
    (Variables|Default|SetOwnerPos (Transformation|GetActorLocation (Components|GetOwner)))
    (Utilities|FlowControl|Sequence
      (:then_0
        (Utilities|FlowControl|DoOnce false
          (:Completed
            (bind _outactors (Actor|GetAllActorsOfClass "/Game/BP/Landscape/Chunk.Chunk_C"))
            (bind _outhits (Collision|MultiSphereTraceByChannel _returnvalue_4 (+ _returnvalue_4 "0.000000,0.000000,500.000000") 2e+03 "TraceTypeQuery5" true _outactors "None"))
            (for _array_element _outhits
              (Utilities|Array|Add (Variables|Default|GetPollutionInRange) (.HitActor (Collision|BreakHitResult _array_element)))))))
      (:then_1
        (Utilities|FlowControl|Delay (Variables|Default|GetTimeBetweenCatch))
        (if (Utilities|IsValid _output)
          (Variables|Default|SetSelectedPollution _output)
          (Variables|Default|SetSelectedPolFirstPos (Transformation|GetActorLocation _output))
          (bind _returnvalue_6 (Game|AddComponentbyClass (Variables|Default|GetSelectedPollution) "/Game/BP/Building/Components/AC_PollutionCatch.AC_PollutionCatch_C"))
          (Default|MovementBeforeDestruction _returnvalue_6 (+ (Transformation|GetActorLocation (Components|GetOwner)) "0.000000,0.000000,200.000000"))
          (Utilities|Array|RemoveIndex (Variables|Default|GetPollutionInRange) _returnvalue_5)
          (Default|RemovePollutionWaste (Variables|Default|GetPollution%20Manager))
          (if (== (Utilities|GetClass _returnvalue_2) "/Game/BP/Building/CB_BuildingPP.CB_BuildingPP_C")
            (bind _ascb_building_pp (Utilities|Casting|CastToCB_BuildingPP _returnvalue_2))
            (Components|Activation|Activate (Variables|/Game/BP/Building/CB_BuildingPP.CB_BuildingPP_C|GetNiagara _ascb_building_pp) false)
            (else
              (bind _ascb_building_net (Utilities|Casting|CastToCB_BuildingNet _returnvalue_2))))
          (elif (> (Utilities|Array|Length (Variables|Default|GetPollutionInRange)) 0)
            (Utilities|Array|RemoveIndex (Variables|Default|GetPollutionInRange) _returnvalue_5))))
      (:then_2
        (Transformation|SetActorRotation (Components|GetOwner) (Math|Rotator|MakeRotator 0.0 0.0 (.yaw (Math|Conversions|RotationFromXVector (Math|Interpolation|VInterpTo (Math|Rotator|GetRotationXVector (Transformation|GetActorRotation (Components|GetOwner))) (Math|Rotator|GetRotationXVector (Math|Rotator|FindLookatRotation (Variables|Default|GetSelectedPolFirstPos) (Variables|Default|GetOwnerPos))) (Utilities|Time|GetWorldDeltaSeconds) 1.0)))))))))