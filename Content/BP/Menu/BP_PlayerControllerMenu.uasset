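; BP_PlayerControllerMenu is the player controller for a menu, forwarding input actions to the menu owned by its HUD.
; On BeginPlay it caches the HUD as BP_HUDMenu, gives focus to the game viewport and hides the mouse cursor.
; The ChangeMenuButton and ChooseBuilding actions call the menu's ChangeButton and ChooseButton, so the menu is operated through input actions without a visible cursor.
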(event EventBeginPlay
  (bind _asbp_hudmenu (Utilities|Casting|CastToBP_HUDMenu (HUD|GetHUD)))
  (Variables|Default|SetAs%20BP%20HUDMenu _asbp_hudmenu)
  (Class|WidgetBlueprintLibrary|SetFocustoGameViewport)
  (Variables|Default|SetbShowMouseCursor false))

(event Input|ActionEvents|InputActionChangeMenuButton
  (params (Key :type Key%20Structure :default "None"))
  (:Pressed
    (Default|ChangeButton (Variables|/Game/BP/Menu/BP_HUDMenu.BP_HUDMenu_C|GetMenu (Variables|Default|GetAs%20BP%20HUDMenu)))))

(event Input|ActionEvents|InputActionChooseBuilding
  (params (Key :type Key%20Structure :default "None"))
  (:Pressed
    (Default|ChooseButton (Variables|/Game/BP/Menu/BP_HUDMenu.BP_HUDMenu_C|GetMenu (Variables|Default|GetAs%20BP%20HUDMenu)))))

(fn ConstructionScript)