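; BP_HUDMenu is the menu HUD Blueprint that shows the menu and handles the switch to the main level.
; On BeginPlay it creates the WP_Menu widget, adds it to the viewport and shows the mouse cursor.
; LoadMainlevel clears all widgets, displays the WP_LoadingMenu loading screen, waits on a short fixed delay, then opens the Main level by object reference.
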(event Custom|LoadMainlevel
  (Viewport|RemoveAllWidgets)
  (bind _returnvalue (UserInterface|CreateWidget "/Game/BP/Menu/WP_LoadingMenu.WP_LoadingMenu_C"))
  (bind _output_get (Variables|Default|SetLoadingScreen _returnvalue))
  (UserInterface|Viewport|AddtoViewport _output_get 0)
  (Utilities|FlowControl|Delay 1.0)
  (Game|OpenLevel(byObjectReference) "/Game/Levels/Main.Main"))

(event EventBeginPlay
  (bind _returnvalue (UserInterface|CreateWidget "/Game/BP/Menu/WP_Menu.WP_Menu_C"))
  (bind _output_get (Variables|Default|SetMenu _returnvalue))
  (UserInterface|Viewport|AddtoViewport _output_get 0)
  (Variables|/Script/Engine.PlayerController|SetbShowMouseCursor (Game|GetPlayerController 0) true))

(fn ConstructionScript)