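; Player controller for a building-placement game with pollution cleanup, routing input to placement, HUD building selection and the pause menu.
; Placement mode spawns a preview actor that follows a mouse-cursor trace and rotates in quarter turns.
; Confirming a valid spot spawns the real building, triggers its fog or water cleaner against the PollutionManager, and registers it with the EntitiesController.
; BeginPlay spawns that EntitiesController, caches references and starts timed music.
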(event EventTick
  (params (DeltaSeconds :type Float%20%28single-precision%29))
  (if (Variables|Default|GetPlacementModeEnabled)
    (CallFunction|UpdatePlacement)))

(event EventBeginPlay
  (bind _asmain_hud (Utilities|Casting|CastToMainHud (HUD|GetHUD)))
  (Variables|Default|SetMainHUD _asmain_hud)
  (Class|WidgetBlueprintLibrary|SetFocustoGameViewport)
  (Variables|Default|SetbShowMouseCursor false)
  (CallFunction|SpawnEntitiesController)
  (bind _returnvalue (Actor|GetActorOfClass "/Game/BP/BP_PollutionManager.BP_PollutionManager_C"))
  (Variables|Default|SetPollutionManager _returnvalue)
  (bind _returnvalue_2 (Actor|GetActorOfClass "/Game/BP/Audio/KoroguAudio.KoroguAudio_C"))
  (Variables|Default|SetKoroguAudio _returnvalue_2)
  (Utilities|FlowControl|Delay 4.0)
  (bind _returnvalue_3 (Audio|SpawnSound2D "/Game/Assets/Audio/Music/Music.Music" 1.0 1.0 0.0 0))
  (Utilities|FlowControl|Delay 9e+02)
  (Audio|Components|Audio|FadeOut _returnvalue_3 1.0 0.0 "Linear" :!class /Script/Engine.AudioComponent))

(event Input|ActionEvents|InputActionChangeMenuButton
  (params (Key :type Key%20Structure :default "None"))
  (:Pressed
    (if (Game|IsGamePaused)
      (Default|ChangeButton (Variables|/Game/UI/MainHud.MainHud_C|GetPauseScreen (Variables|Default|GetMainHUD))))))

(event Input|ActionEvents|InputActionPauseGame
  (params (Key :type Key%20Structure :default "None"))
  (bind _mainhud (Variables|Default|GetMainHUD))
  (:Pressed
    (if (Game|IsGamePaused)
      (Default|PauseEnd _mainhud)
      (Game|SetGamePaused false)
      (else
        (Default|PauseStart _mainhud)
        (Game|SetGamePaused true)))))

(event Input|ActionEvents|InputActionMouseLeftClick
  (params (Key :type Key%20Structure :default "None"))
  (:Pressed
    (if (Variables|Default|GetPlacementModeEnabled)
      (CallFunction|SpawnBuilding)
      (Default|NewBuilding (Variables|Default|GetEntitiesController) (Variables|Default|GetConstructedBuidling) (Variables|Default|GetPollutionManager))
      (Class|BPIGA|SpawnPlantesAutour(Message) (Variables|Default|GetConstructedBuidling)))))

(event Input|ActionEvents|InputActionRotateBuilding
  (params (Key :type Key%20Structure :default "None"))
  (:Pressed
    (if (Variables|Default|GetPlacementModeEnabled)
      (CallFunction|RotateBuilding))))

(event Input|ActionEvents|InputActionPlaceBuilding
  (params (Key :type Key%20Structure :default "None"))
  (:Pressed
    (CallFunction|SetPlacementModeEnabled true (Variables|Default|GetBuildingType))))

(event Input|ActionEvents|InputActionChooseBuilding
  (params (Key :type Key%20Structure :default "None"))
  (bind _mainhud (Variables|Default|GetMainHUD))
  (bind _tophudwidget (Variables|/Game/UI/MainHud.MainHud_C|GetTopHudWidget _mainhud))
  (bind _mainhudwidget (Variables|/Game/UI/WBP_Main.WBP_Main_C|GetMainHudWidget _tophudwidget))
  (:Pressed
    (if (Game|IsGamePaused)
      (Default|ChooseButton (Variables|/Game/UI/MainHud.MainHud_C|GetPauseScreen (Variables|Default|GetMainHUD)))
      (elif (Variables|/Game/UI/MainHudWidget.MainHudWidget_C|GetIsSelectingBuilding _mainhudwidget)
        (if (Variables|Default|GetPlacementModeEnabled)
          (CallFunction|SpawnBuilding)
          (Default|NewBuilding (Variables|Default|GetEntitiesController) (Variables|Default|GetConstructedBuidling) (Variables|Default|GetPollutionManager))
          (Class|BPIGA|SpawnPlantesAutour(Message) (Variables|Default|GetConstructedBuidling))
          (else
            (Default|ClickButton _mainhudwidget)))
        (else
          (Default|ChooseBuilding _mainhudwidget))))))

(event Input|ActionEvents|InputActionChangeBuildingRight
  (params (Key :type Key%20Structure :default "None"))
  (:Pressed
    (if (Game|IsGamePaused)
      (Default|ChangeButton (Variables|/Game/UI/MainHud.MainHud_C|GetPauseScreen (Variables|Default|GetMainHUD)))
      (else
        (Default|ChangeBuilding (Variables|/Game/UI/WBP_Main.WBP_Main_C|GetMainHudWidget (Variables|/Game/UI/MainHud.MainHud_C|GetTopHudWidget (Variables|Default|GetMainHUD))) 1)))))

(event Input|ActionEvents|InputActionChangeBuildingLeft
  (params (Key :type Key%20Structure :default "None"))
  (:Pressed
    (if (Game|IsGamePaused)
      (Default|ChangeButton (Variables|/Game/UI/MainHud.MainHud_C|GetPauseScreen (Variables|Default|GetMainHUD)))
      (else
        (Default|ChangeBuilding (Variables|/Game/UI/WBP_Main.WBP_Main_C|GetMainHudWidget (Variables|/Game/UI/MainHud.MainHud_C|GetTopHudWidget (Variables|Default|GetMainHUD))) -1)))))

(event Input|ActionEvents|InputActionMouseRightClick
  (params (Key :type Key%20Structure :default "None"))
  (:Pressed
    (if (Variables|Default|GetPlacementModeEnabled)
      (Variables|Default|SetPlacementModeEnabled false)
      (Actor|DestroyActor (Variables|Default|GetPlaceableActor)))))

(fn ConstructionScript)

(fn SetPlacementModeEnabled
  (params (IsEnabled :type Boolean) (BuildingID :type Integer))
  (if (== IsEnabled (Variables|Default|GetPlacementModeEnabled))
    (return)
    (else
      (bind _output_get (Variables|Default|SetPlacementModeEnabled IsEnabled))
      (if _output_get
        (bind _returnvalue (Game|SpawnActorfromClass (Utilities|Array|Get(acopy) (Variables|Default|GetPlaceableActorType) BuildingID) (Math|Transform|MakeTransform "0.000000,0.000000,-100000.000000") "AlwaysSpawn" "MultiplyWithRoot" 0 0))
        (bind _output_get_2 (Variables|Default|SetPlaceableActor _returnvalue))
        (Utilities|IsValid (Actor|GetComponentbyClass _output_get_2 "/Game/BP/Building/Components/CB_ClickableComponent.CB_ClickableComponent_C")
          (:Is%20Valid
            (Default|InPlacementMode (Actor|GetComponentbyClass _output_get_2 "/Game/BP/Building/Components/CB_ClickableComponent.CB_ClickableComponent_C")))
          (:Is%20Not%20Valid
            _))
        (AddComponent|AddCBPloppableComponent _output_get_2)
        (else
          (Utilities|IsValid (Variables|Default|GetPlaceableActor)
            (:Is%20Valid
              (Actor|DestroyActor (Variables|Default|GetPlaceableActor)))))))))

(fn UpdatePlacement
  (bind (_worldlocation _worlddirection) (Game|Player|ConvertMouseLocationToWorldSpace))
  (bind _placeableactor (Variables|Default|GetPlaceableActor))
  (bind _outhit (Collision|LineTraceByChannel _worldlocation (+ _worldlocation (* _worlddirection 1e+04)) "TraceTypeQuery2" false 0 "None"))
  (if (.bBlockingHit (Collision|BreakHitResult _outhit))
    (Transformation|SetActorLocation _placeableactor (Math|Vector|MakeVector (.X (Math|Vector|BreakVector (.ImpactPoint (Collision|BreakHitResult _outhit)))) (.Y (Math|Vector|BreakVector (.ImpactPoint (Collision|BreakHitResult _outhit)))) (+ (.Z (Math|Vector|BreakVector (.BoxExtent (Collision|GetActorBounds _placeableactor false false)))) (.Z (Math|Vector|BreakVector (.ImpactPoint (Collision|BreakHitResult _outhit)))))) false false)))

(fn SpawnBuilding
  (bind _placeableactor (Variables|Default|GetPlaceableActor))
  (bind _koroguaudio (Variables|Default|GetKoroguAudio))
  (bind _returnvalue (Actor|GetComponentbyClass _placeableactor "/Game/BP/Building/Components/CB_PloppableComponent.CB_PloppableComponent_C"))
  (Utilities|IsValid _returnvalue
    (:Is%20Valid
      (if (Variables|/Game/BP/Building/Components/CB_PloppableComponent.CB_PloppableComponent_C|GetIsPlacementValid _returnvalue)
        (Utilities|IsValid _koroguaudio
          (:Is%20Valid
            (Default|PlayKoroguVL _koroguaudio))
          (:Is%20Not%20Valid
            _))
        (bind _returnvalue_2 (Game|SpawnActorfromClass (Utilities|Array|Get(acopy) (Variables|Default|GetPlaceableActorType) (Variables|Default|GetBuildingType)) (Transformation|GetActorTransform (Variables|Default|GetPlaceableActor)) "AlwaysSpawn" "MultiplyWithRoot" 0 0))
        (bind _output_get (Variables|Default|SetConstructedBuidling _returnvalue_2))
        (CallFunction|SetPlacementModeEnabled false (Variables|Default|GetBuildingType))
        (bind _ascb_building_asset (Utilities|Casting|CastToCB_BuildingAsset _output_get))
        (Variables|/Game/BP/Building/CB_BuildingAsset.CB_BuildingAsset_C|SetIsPlaced _ascb_building_asset true)
        (Utilities|IsValid (Actor|GetComponentbyClass _ascb_building_asset "/Game/BP/Building/Components/AC_FogCleaner.AC_FogCleaner_C")
          (:Is%20Valid
            (Default|CheckFog (Actor|GetComponentbyClass _ascb_building_asset "/Game/BP/Building/Components/AC_FogCleaner.AC_FogCleaner_C") (Variables|Default|GetPollutionManager)))
          (:Is%20Not%20Valid
            (Utilities|IsValid (Actor|GetComponentbyClass _ascb_building_asset "/Game/BP/Building/Components/AC_WaterPollutionCleaner.AC_WaterPollutionCleaner_C")
              (:Is%20Valid
                (Default|CheckWaterPollution (Actor|GetComponentbyClass _ascb_building_asset "/Game/BP/Building/Components/AC_WaterPollutionCleaner.AC_WaterPollutionCleaner_C") (Variables|Default|GetPollutionManager))))))))))

(fn RotateBuilding
  (Transformation|AddActorLocalRotation (Variables|Default|GetPlaceableActor) (Math|Rotator|MakeRotator 0.0 0.0 9e+01) false false))

(fn SpawnEntitiesController
  (bind _returnvalue (Game|SpawnActorfromClass "/Game/BP/Entity/BP_EntitiesController.BP_EntitiesController_C" (Math|Transform|MakeTransform "0, 0, 0") "Undefined" "MultiplyWithRoot" 0 0))
  (Variables|Default|SetEntitiesController _returnvalue))

(fn ChangeBuildingColor
  (params (CB_BuildingAsset :type CB%20Building%20Asset%20Object%20Reference)))