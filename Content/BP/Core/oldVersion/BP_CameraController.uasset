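; Camera controller Blueprint, filed under an old-version folder, that provides orbit, planar movement and zoom for a spring-arm camera.
; Orbit input adds scaled controller yaw, and forward and strafe inputs add movement along directions derived from that yaw alone, ignoring pitch and roll.
; Zoom input adjusts the spring arm length by a speed factor, clamped to a fixed range.
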(event Custom|CameraZoom
  (params (Magnitude :type Float%20%28double-precision%29))
  (bind _springarm (Variables|Default|GetSpringArm))
  (Variables|/Script/Engine.SpringArmComponent|SetTargetArmLength _springarm (Math|Float|Clamp(Float) (+ (* Magnitude (Variables|Default|GetZoomSpeed)) (Variables|/Script/Engine.SpringArmComponent|GetTargetArmLength _springarm)) 3e+02 2e+03)))

(event Custom|MoveForward
  (params (Magnitude :type Float%20%28double-precision%29))
  (Pawn|Input|AddMovementInput (Math|Vector|GetForwardVector (Math|Rotator|MakeRotator 0.0 0.0 (.Yaw (Math|Rotator|BreakRotator (Pawn|GetControlRotation :!class /Script/Engine.Pawn))))) Magnitude false))

(event Custom|LeftRightStrafe
  (params (Magnitude :type Float%20%28double-precision%29))
  (Pawn|Input|AddMovementInput (Math|Vector|GetRightVector (Math|Rotator|MakeRotator 0.0 0.0 (.Yaw (Math|Rotator|BreakRotator (Pawn|GetControlRotation :!class /Script/Engine.Pawn))))) Magnitude false))

(event Custom|CameraOrbit
  (params (Magnitude :type Float%20%28double-precision%29))
  (Pawn|Input|AddControllerYawInput (* Magnitude (Variables|Default|GetOrbitSpeed))))

(fn ConstructionScript)