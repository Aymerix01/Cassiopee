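; Player controller for a building game that forwards camera input to the CB_CameraController pawn and handles mouse-driven building placement.
; Placement mode moves a preview actor along a cursor trace, supports rotation, and spawns the building on click when valid.
; That click also sends entities spawned at BeginPlay around the traced actor's bounds.
; Outside placement, Tick polls until all entities arrive or stall, then flags their AI controllers as arrived.
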(event EventTick
  (params (DeltaSeconds :type Float%20%28single-precision%29))
  (if (Variables|Default|GetPlacementModeEnabled)
    (CallFunction|UpdatePlacement)
    (elif (not (Variables|Default|GetAllEntityArrivedToBuild))
      (CallFunction|EntityArrivedtoBuild))))

(event EventBeginPlay
  (CallFunction|SpawnEntity)
  (Variables|Default|SetAllEntityArrivedToBuild true))

(event Input|ActionEvents|InputActionCameraZoomIn
  (params (Key :type Key%20Structure))
  (:Pressed
    (bind _ascb_camera_controller (Utilities|Casting|CastToCB_CameraController (Pawn|GetControlledPawn)))
    (Default|CameraZoom _ascb_camera_controller -1.0)))

(event Input|ActionEvents|InputActionCameraZoomOut
  (params (Key :type Key%20Structure))
  (:Pressed
    (bind _ascb_camera_controller (Utilities|Casting|CastToCB_CameraController (Pawn|GetControlledPawn)))
    (Default|CameraZoom _ascb_camera_controller 1.0)))

(event Input|ActionEvents|InputActionMouseLeftClick
  (params (Key :type Key%20Structure))
  (:Pressed
    (if (Variables|Default|GetPlacementModeEnabled)
      (CallFunction|SpawnBuilding)
      (CallFunction|MoveEntity)
      (CallFunction|EntityArrivedtoBuild))))

(event Input|ActionEvents|InputActionRotateBuilding
  (params (Key :type Key%20Structure))
  (:Pressed
    (if (Variables|Default|GetPlacementModeEnabled)
      (CallFunction|RotateBuilding))))

(event Input|ActionEvents|InputActionPlaceBuilding
  (params (Key :type Key%20Structure))
  (:Pressed
    (CallFunction|SetPlacementModeEnabled true)))

(event Input|AxisEvents|InputAxisCameraOrbit
  (params (AxisValue :type Float%20%28single-precision%29))
  (bind _ascb_camera_controller (Utilities|Casting|CastToCB_CameraController (Pawn|GetControlledPawn)))
  (Default|CameraOrbit _ascb_camera_controller AxisValue))

(event Input|AxisEvents|InputAxisMoveForward/Backward
  (params (AxisValue :type Float%20%28single-precision%29))
  (bind _ascb_camera_controller (Utilities|Casting|CastToCB_CameraController (Pawn|GetControlledPawn)))
  (Default|MoveForward _ascb_camera_controller AxisValue))

(event Input|AxisEvents|InputAxisStrafeLeft/Right
  (params (AxisValue :type Float%20%28single-precision%29))
  (bind _ascb_camera_controller (Utilities|Casting|CastToCB_CameraController (Pawn|GetControlledPawn)))
  (Default|LeftRightStrafe _ascb_camera_controller AxisValue))

(fn ConstructionScript)

(fn SetPlacementModeEnabled
  (params (IsEnabled :type Boolean))
  (if (== IsEnabled (Variables|Default|GetPlacementModeEnabled))
    (return)
    (else
      (bind _output_get (Variables|Default|SetPlacementModeEnabled IsEnabled))
      (if _output_get
        (bind _returnvalue (Game|SpawnActorfromClass (Variables|Default|GetPlaceableActorType) (Math|Transform|MakeTransform "0.000000,0.000000,-100000.000000") "AlwaysSpawn" "MultiplyWithRoot" 0 0))
        (bind _output_get_2 (Variables|Default|SetPlaceableActor _returnvalue))
        (Utilities|IsValid (Actor|GetComponentbyClass _output_get_2 "/Game/BP/Building/Components/CB_ClickableComponent.CB_ClickableComponent_C")
          (:Is%20Valid
            (Default|InPlacementMode (Actor|GetComponentbyClass _output_get_2 "/Game/BP/Building/Components/CB_ClickableComponent.CB_ClickableComponent_C")))
          (:Is%20Not%20Valid
            _))
        (AddComponent|AddCBPloppableComponent _output_get_2)
        (else
          (Utilities|IsValid (Variables|Default|GetPlaceableActor)
            (:Is%20Valid
              (Actor|DestroyActor (Variables|Default|GetPlaceableActor)))))))))

(fn UpdatePlacement
  (bind (_worldlocation _worlddirection) (Game|Player|ConvertMouseLocationToWorldSpace))
  (bind _placeableactor (Variables|Default|GetPlaceableActor))
  (bind _outhit (Collision|LineTraceByChannel _worldlocation (+ _worldlocation (* _worlddirection 1e+04)) "TraceTypeQuery3" false 0 "None"))
  (if (.bBlockingHit (Collision|BreakHitResult _outhit))
    (Transformation|SetActorLocation _placeableactor (Math|Vector|MakeVector (.X (Math|Vector|BreakVector (.ImpactPoint (Collision|BreakHitResult _outhit)))) (.Y (Math|Vector|BreakVector (.ImpactPoint (Collision|BreakHitResult _outhit)))) (+ (.Z (Math|Vector|BreakVector (.BoxExtent (Collision|GetActorBounds _placeableactor false false)))) (.Z (Math|Vector|BreakVector (.ImpactPoint (Collision|BreakHitResult _outhit)))))) false false)))

(fn SpawnBuilding
  (bind _placeableactor (Variables|Default|GetPlaceableActor))
  (bind _returnvalue (Actor|GetComponentbyClass _placeableactor "/Game/BP/Building/Components/CB_PloppableComponent.CB_PloppableComponent_C"))
  (Utilities|IsValid _returnvalue
    (:Is%20Valid
      (if (Variables|/Game/BP/Building/Components/CB_PloppableComponent.CB_PloppableComponent_C|GetIsPlacementValid _returnvalue)
        (Game|SpawnActorfromClass (Variables|Default|GetPlaceableActorType) (Transformation|GetActorTransform (Variables|Default|GetPlaceableActor)) "AlwaysSpawn" "MultiplyWithRoot" 0 0)
        (CallFunction|SetPlacementModeEnabled false)))))

(fn RotateBuilding
  (Transformation|AddActorLocalRotation (Variables|Default|GetPlaceableActor) (Math|Rotator|MakeRotator 0.0 0.0 9e+01) false false))

(fn SpawnEntity
  (for _index (range 0 9)
    (bind _returnvalue (Game|SpawnActorfromClass "/Game/BP/Entity/oldVersion/BP_MyEntity.BP_MyEntity_C" (Math|Transform|MakeTransform (Math|Vector|MakeVector (+ (* _index (Math|Float|MakeLiteralFloat 2e+02)) (Math|Float|MakeLiteralFloat 1.2e+03)) 0.0 0.0)) "Undefined" "MultiplyWithRoot" 0 0))
    (Utilities|Array|Add (Variables|Default|GetEntitiesSpawned) _returnvalue)))

(fn MoveEntity
  (bind _returnvalue (Game|GetPlayerController 0))
  (bind (_worldlocation _worlddirection) (Game|Player|ConvertMouseLocationToWorldSpace _returnvalue))
  (bind _outhit (Collision|LineTraceByChannel (Transformation|GetWorldLocation (Actor|GetComponentbyClass (Pawn|GetControlledPawn) "/Script/Engine.CameraComponent")) (+ _worldlocation (* _worlddirection (+ (Math|Vector|GetForwardVector (Pawn|GetControlRotation _returnvalue :!class /Script/Engine.Controller)) (Math|Float|MakeLiteralFloat 1e+06)))) "TraceTypeQuery1" false 0 "None"))
  (for (_array_element _array_index) (Variables|Default|GetEntitiesSpawned)
    (bind _asbp_my_entity_controller (Utilities|Casting|CastToBP_MyEntityController (Pawn|GetController _array_element)))
    (bind _returnvalue_2 (Class|MyEntityController|PlaceActorAroundBounds _asbp_my_entity_controller (.Origin (Collision|GetActorBounds (.HitActor (Collision|BreakHitResult _outhit)) false false)) (.BoxExtent (Collision|GetActorBounds (.HitActor (Collision|BreakHitResult _outhit)) false false)) (Math|Conversions|ToFloat(Integer) _array_index) (Math|Conversions|ToFloat(Integer) (Utilities|Array|Length (Variables|Default|GetEntitiesSpawned)))))
    (Class|MyEntityController|TraveltoNewBuilding _asbp_my_entity_controller _returnvalue_2)))

(fn EntityArrivedtoBuild
  (Variables|Default|SetAllEntityArrivedToBuild true)
  (for _array_element (Variables|Default|GetEntitiesSpawned)
    (bind _asbp_my_entity_controller (Utilities|Casting|CastToBP_MyEntityController (Pawn|GetController _array_element)))
    (if (not (or (Class|MyEntityController|IsMotionlessforSomeTime _asbp_my_entity_controller (Variables|/Script/Cassiopee.MyEntityController|GettimeBeforeMotionless _asbp_my_entity_controller)) (Class|MyEntityController|HasReachedDestination _asbp_my_entity_controller (Variables|/Script/Cassiopee.MyEntityController|GetIADestination _asbp_my_entity_controller))))
      (Variables|Default|SetAllEntityArrivedToBuild false)))
  (if (Variables|Default|GetAllEntityArrivedToBuild)
    (for _array_element_2 (Variables|Default|GetEntitiesSpawned)
      (bind _asbp_my_entity_controller_2 (Utilities|Casting|CastToBP_MyEntityController (Pawn|GetController _array_element_2)))
      (Variables|/Script/Cassiopee.MyEntityController|SetIsArrivedToBuild _asbp_my_entity_controller_2 true))))