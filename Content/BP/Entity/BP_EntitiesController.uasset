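; Entity controller that spawns worker AI pawns at start and coordinates them to construct player buildings.
; SendEntitiesBuild picks the nearest free entities up to the building's required count and dispatches them.
; CheckAllEntitiesArrived completes construction once all arrive, then triggers the building's fog, water, Korogu or pollution-watcher component.
; InitBuildingPollution counts spawned buildings to advance HUD tutorial and unlock stages.
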(event Custom|NewBuilding
  (params (Building :type Actor%20Object%20Reference) (PollutionManager :type BP%20Pollution%20Manager%20Object%20Reference))
  (bind _ascb_building_asset (Utilities|Casting|CastToCB_BuildingAsset Building))
  (Default|Build _ascb_building_asset Building PollutionManager))

(event Custom|InitBuildingPollution
  (params (Building :type Actor%20Object%20Reference))
  (bind _returnvalue (Utilities|GetClass Building))
  (Variables|Default|SetNbrBuildingSpawned (+ (Variables|Default|GetNbrBuildingSpawned) 1))
  (if (< (Variables|Default|GetNbrBuildingSpawned) 9)
    (if (== _returnvalue "/Game/BP/Building/CB_BuildingEA.CB_BuildingEA_C")
      (Utilities|FlowControl|DoOnce false
        (:Completed
          (bind _asmain_hud (Utilities|Casting|CastToMainHud (HUD|GetHUD (Game|GetPlayerController 0))))
          (Default|InitPollutionBuildings (Variables|/Game/UI/WBP_Main.WBP_Main_C|GetMainHudWidget (Variables|/Game/UI/MainHud.MainHud_C|GetTopHudWidget _asmain_hud))))))
    (elif (< (Utilities|Array|Length (Variables|Default|GetEntitiesControllerSpawned)) 19)
      (Utilities|FlowControl|DoOnce false
        (:Completed
          (bind _asmain_hud_2 (Utilities|Casting|CastToMainHud (HUD|GetHUD (Game|GetPlayerController 0))))
          (Default|InitHospital (Variables|/Game/UI/WBP_Main.WBP_Main_C|GetMainHudWidget (Variables|/Game/UI/MainHud.MainHud_C|GetTopHudWidget _asmain_hud_2)))))
      (elif (== _returnvalue "/Game/BP/Building/CB_BuildingPW.CB_BuildingPW_C")
        (bind _asmain_hud_3 (Utilities|Casting|CastToMainHud (HUD|GetHUD (Game|GetPlayerController 0))))
        (Default|FinAide (Variables|/Game/UI/WBP_Main.WBP_Main_C|GetMainHudWidget (Variables|/Game/UI/MainHud.MainHud_C|GetTopHudWidget _asmain_hud_3)))
        (else
          (Utilities|FlowControl|DoOnce false
            (:Completed
              (bind _asmain_hud_4 (Utilities|Casting|CastToMainHud (HUD|GetHUD (Game|GetPlayerController 0))))
              (Default|InitPollutionManager (Variables|/Game/UI/WBP_Main.WBP_Main_C|GetMainHudWidget (Variables|/Game/UI/MainHud.MainHud_C|GetTopHudWidget _asmain_hud_4)))
              (Utilities|FlowControl|Delay 6e+01)
              (Default|InitLastBuildings (Variables|/Game/UI/WBP_Main.WBP_Main_C|GetMainHudWidget (Variables|/Game/UI/MainHud.MainHud_C|GetTopHudWidget _asmain_hud_4))))))))))

(event EventBeginPlay
  (for _index (range 1 (Variables|Default|GetInitialEntitiesNumber))
    (CallFunction|SpawnEntity (Math|Vector|MakeVector (Math|Random|RandomFloatinRange -1e+03 1e+03) (Math|Random|RandomFloatinRange -1e+03 1e+03) 1e+03))))

(fn ConstructionScript)

(fn SpawnEntity
  (params (Location :type Vector))
  (bind _returnvalue (Math|Transform|MakeTransform Location))
  (bind _returnvalue_2 (AI|SpawnAIFromClass "/Game/BP/Entity/BP_Entity.BP_Entity_C" 0 (.location _returnvalue) (.rotation _returnvalue) true 0))
  (Utilities|IsValid _returnvalue_2
    (:Is%20Valid
      (bind _asbp_entity_controller (Utilities|Casting|CastToBP_EntityController (Pawn|GetController _returnvalue_2)))
      (Utilities|Array|Add (Variables|Default|GetEntitiesControllerSpawned) _asbp_entity_controller))
    (:Is%20Not%20Valid
      (Development|PrintString "WARNING : Error spawn Entity" true true "(R=1.000000,G=0.010417,B=0.010417,A=1.000000)")
      (Development|PrintString "May cause some building issues" true true "(R=1.000000,G=0.076232,B=0.000000,A=1.000000)"))))

(fn SendEntitiesBuild
  (params (Building :type Actor%20Object%20Reference))
  (bind _distancebuildingentity1 (LocalVariables|GetDistanceBuildingEntity1))
  (bind _entitiescontrollerspawned (Variables|Default|GetEntitiesControllerSpawned))
  (bind _indexofminvalue (Math|Float|MinOfFloatArray _distancebuildingentity1))
  (bind _output (Utilities|Array|Get(acopy) _entitiescontrollerspawned _indexofminvalue))
  (Utilities|IsValid Building
    (:Is%20Valid
      (bind _ascb_building_asset (Utilities|Casting|CastToCB_BuildingAsset Building))
      (LocalVariables|SetNumberEntitiesNecessary (Variables|/Game/BP/Building/CB_BuildingAsset.CB_BuildingAsset_C|GetNumberEntities _ascb_building_asset))
      (LocalVariables|SetNumberEntitiesSpawned (Utilities|Array|Length (Variables|Default|GetEntitiesControllerSpawned)))
      (if (< (LocalVariables|GetNumberEntitiesNecessary) (LocalVariables|GetNumberEntitiesSpawned))
        (for _array_element (Variables|Default|GetEntitiesControllerSpawned)
          (Utilities|Array|Add (LocalVariables|GetDistanceBuildingEntity1) (Transformation|GetDistanceTo Building (Pawn|GetControlledPawn _array_element))))
        (Utilities|FlowControl|ForLoopwithBreak 1 (LocalVariables|GetNumberEntitiesSpawned) :!label _label
          (:LoopBody
            (if (Variables|/Game/BP/Entity/BP_EntityController.BP_EntityController_C|GetIsBuilding _output)
              _
              (else
                (Variables|/Game/BP/Entity/BP_EntityController.BP_EntityController_C|SetIsArrived _output false)
                (Variables|/Game/BP/Entity/BP_EntityController.BP_EntityController_C|SetIsBuilding _output true)
                (Utilities|Array|Add (LocalVariables|GetEntitiesControllerBuilding) _output)))
            (Utilities|Array|SetArrayElem (LocalVariables|GetDistanceBuildingEntity1) _indexofminvalue 1e+21)
            (if (== (Utilities|Array|Length (LocalVariables|GetEntitiesControllerBuilding)) (LocalVariables|GetNumberEntitiesNecessary))
              (goto _label Break)))
          (:Completed
            (if (== (Utilities|Array|Length (LocalVariables|GetEntitiesControllerBuilding)) (LocalVariables|GetNumberEntitiesNecessary))
              (for _array_element_2 (LocalVariables|GetEntitiesControllerBuilding)
                (Variables|/Game/BP/Entity/BP_EntityController.BP_EntityController_C|SetBuildng _array_element_2 Building)
                (Default|ChangeIsBuilding _array_element_2 true))
              (return true (LocalVariables|GetEntitiesControllerBuilding))
              (else
                (return false 0)))))
        (else
          (return false 0))))))

(fn CheckAllEntitiesArrived
  (params (EntitiesControllerBuilding :type Array%20of%20BP%20Entity%20Controller%20Object%20References) (Building :type Actor%20Object%20Reference) (PollutionManager :type BP%20Pollution%20Manager%20Object%20Reference))
  (bind _returnvalue (Actor|GetComponentbyClass Building "/Game/BP/Building/Components/AC_FogCleaner.AC_FogCleaner_C"))
  (bind _returnvalue_2 (Actor|GetComponentbyClass Building "/Game/BP/Building/Components/AC_PollutionWatcher.AC_PollutionWatcher_C"))
  (bind _returnvalue_3 (Actor|GetComponentbyClass Building "/Game/BP/Building/Components/AC_WaterPollutionCleaner.AC_WaterPollutionCleaner_C"))
  (bind _returnvalue_4 (Actor|GetComponentbyClass Building "/Game/BP/Building/Components/AC_KoroguSpawner.AC_KoroguSpawner_C"))
  (LocalVariables|SetIsEveryEntitiesArrived true)
  (bind _array_element (Utilities|Array|ForEachLoopwithBreak EntitiesControllerBuilding)
    (:LoopBody
      (if (not (Variables|/Game/BP/Entity/BP_EntityController.BP_EntityController_C|GetIsArrived _array_element))
        (LocalVariables|SetIsEveryEntitiesArrived false)
        (Default|ChangeIsBuilding _array_element true)))
    (:Completed
      (if (LocalVariables|GetIsEveryEntitiesArrived)
        (for _array_element_2 EntitiesControllerBuilding
          (Variables|/Game/BP/Entity/BP_EntityController.BP_EntityController_C|SetIsArrived _array_element_2 false)
          (Variables|/Game/BP/Entity/BP_EntityController.BP_EntityController_C|SetIsBuilding _array_element_2 false)
          (Default|ChangeIsBuilding _array_element_2 false))
        (bind _ascb_building_asset (Utilities|Casting|CastToCB_BuildingAsset Building)
          (:then
            (Variables|/Game/BP/Building/CB_BuildingAsset.CB_BuildingAsset_C|SetIsConstructed _ascb_building_asset true)
            (Default|ChangeBuildingColor _ascb_building_asset)
            (Class|BPIGA|SpawnPlantesAutour(Message) Building)
            (Utilities|IsValid _returnvalue
              (:Is%20Valid
                (Default|CheckFog _returnvalue PollutionManager)
                (return true))
              (:Is%20Not%20Valid
                (Utilities|IsValid _returnvalue_3
                  (:Is%20Valid
                    (Default|CheckWaterPollution _returnvalue_3 PollutionManager)
                    (return true))
                  (:Is%20Not%20Valid
                    (Utilities|IsValid _returnvalue_4
                      (:Is%20Valid
                        (Default|SpawnKorogu _returnvalue_4)
                        (return true))
                      (:Is%20Not%20Valid
                        (Utilities|IsValid _returnvalue_2
                          (:Is%20Valid
                            (Default|InitPollutionWatcher _returnvalue_2))
                          (:Is%20Not%20Valid
                            _))
                        (return true))))))))
          (:CastFailed
            (return false)))
        (else
          (return false))))))